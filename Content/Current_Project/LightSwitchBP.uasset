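; Light switch actor that ends the game when the player presses E inside its trigger box.
; Box overlap caches the first-person character and enables input on the actor, and leaving the box disables it.
; E has the game mode refresh its lights array and trample the lights, triggers the player's flashlight trample message with zero end intensity, then quits after a short delay.
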(event `Key|E`
  (params (Key :type "Key Structure"))
  (:`Pressed`
    (bind _asfirst_person_game_mode (cast `/Game/FirstPersonBP/Blueprints/FirstPersonGameMode` (`GameplayStatics.GetGameMode`)))
    (`/Game/FirstPersonBP/Blueprints/FirstPersonGameMode.UpdateLightsArray` _asfirst_person_game_mode)
    (`/Game/FirstPersonBP/Blueprints/FirstPersonGameMode.TrampleLights` _asfirst_person_game_mode 0.0)
    (message `/Game/Current_Project/TeleportInter.TrampleFlashlight` (`self.Player`) 5 0.0)
    (`KismetSystemLibrary.Delay` 2.0)
    (`KismetSystemLibrary.QuitGame` null "Quit")))

(event `self.Box.OnComponentBeginOverlap`
  (params (OverlappedComponent :type "PrimitiveComponent Object Reference") (OtherActor :type "Actor Object Reference") (OtherComp :type "PrimitiveComponent Object Reference") (OtherBodyIndex :type Integer) (bFromSweep :type Boolean) (SweepResult :type "HitResult Structure (by ref)"))
  (if (not (== (`self.Player`) "/Game/FirstPersonBP/Blueprints/FirstPersonCharacter_3.FirstPersonCharacter_3"))
    (bind _asfirst_person_character_3 (cast `/Game/FirstPersonBP/Blueprints/FirstPersonCharacter_3` OtherActor))
    (set `self.Player` _asfirst_person_character_3))
  (`self.EnableInput` (`GameplayStatics.GetPlayerController` 0)))

(event `self.Box.OnComponentEndOverlap`
  (params (OverlappedComponent :type "PrimitiveComponent Object Reference") (OtherActor :type "Actor Object Reference") (OtherComp :type "PrimitiveComponent Object Reference") (OtherBodyIndex :type Integer))
  (`self.DisableInput` (`GameplayStatics.GetPlayerController` 0)))

(fn `UserConstructionScript`)